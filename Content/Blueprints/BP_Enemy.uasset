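; BP_Enemy is an enemy character that patrols back and forth, walking forward continuously and turning around at floor edges.
; Each Tick adds forward movement input and sphere-traces downward from the LineTraceFloorPos component to detect floor.
; When the floor is lost, a DoOnce, reset once floor is found again, stops movement and rotates the actor 180 degrees through a FlipFlop with identical branches.
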(event Custom|Move%20Forward
  (Pawn|Input|AddMovementInput (Transformation|GetActorForwardVector) 1.0 false))

(event EventTick
  (params (DeltaSeconds :type Float%20%28single-precision%29))
  (bind _charactermovement (Variables|Character|GetCharacterMovement))
  (Utilities|FlowControl|Sequence
    (:then_0
      (bind _floor_detected (CallFunction|LineTraceforFloor))
      (if _floor_detected
        (goto _label Reset)
        (else
          (Utilities|FlowControl|DoOnce false :!label _label
            (:Completed
              (Utilities|FlowControl|FlipFlop
                (:A
                  (Components|Movement|StopMovementImmediately _charactermovement)
                  (Class|Actor|AddActorWorldRotation "0.000000,180.000000,0.000000"))
                (:B
                  (Components|Movement|StopMovementImmediately _charactermovement)
                  (Class|Actor|AddActorWorldRotation "0.000000,180.000000,0.000000"))))))))
    (:then_1
      (CallFunction|MoveForward))))

(fn ConstructionScript)

(fn LineTraceforFloor
  (bind _linetrace_floor_pos (Variables|Default|GetLineTrace%20Floor%20Pos))
  (bind _returnvalue (Transformation|GetWorldLocation _linetrace_floor_pos))
  (bind _returnvalue_2 (Collision|SphereTraceByChannel _returnvalue (+ _returnvalue (* (Math|Vector|GetUpVector (Transformation|GetActorRotation)) -1e+02)) 15.0 "TraceTypeQuery1" false 0 "None" true "(R=1.000000,G=0.000000,B=0.000000,A=1.000000)" "(R=0.000000,G=1.000000,B=0.000000,A=1.000000)" 0.1))
  (return _returnvalue_2))